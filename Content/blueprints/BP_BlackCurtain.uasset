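; BP_BlackCurtain is a static mesh curtain whose opacity fades through OpenCurtain and CloseCurtain events.
; The construction script applies a dynamic instance of M_BlackCourtain to the mesh with Opacity at zero, and BeginPlay raises it to fully opaque.
; Each event plays its own timeline from the start, writing the timeline's Factor into the material's Opacity on every update.
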(event `self.ReceiveBeginPlay`
  (`MaterialInstanceDynamic.SetScalarParameterValue` (`self.DynamicMaterial`) "Opacity" 1.0))

(event `OpenCurtain`
  (bind (_direction _factor) (`Timeline|OpenCurtainTimeline` :!via `PlayFromStart`)
    (:`Update`
      (`MaterialInstanceDynamic.SetScalarParameterValue` (`self.DynamicMaterial`) "Opacity" _factor))))

(event `CloseCurtain`
  (bind (_direction _factor) (`Timeline|CloseCurtainTimeline` :!via `PlayFromStart`)
    (:`Update`
      (`MaterialInstanceDynamic.SetScalarParameterValue` (`self.DynamicMaterial`) "Opacity" _factor))))

(fn `UserConstructionScript`
  (bind _returnvalue (`KismetMaterialLibrary.CreateDynamicMaterialInstance` "/Game/materials/M_BlackCourtain.M_BlackCourtain"))
  (bind _output_get (set `self.DynamicMaterial` _returnvalue))
  (`PrimitiveComponent.SetMaterial` (`self.StaticMeshComponent`) 0 _output_get)
  (`MaterialInstanceDynamic.SetScalarParameterValue` _output_get "Opacity" 0.0))