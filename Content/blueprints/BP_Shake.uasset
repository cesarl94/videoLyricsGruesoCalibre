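; BP_Shake is an actor whose static mesh jitters randomly around its starting position.
; BeginPlay caches the mesh's world location, and every Tick places it at that origin plus a random offset per axis.
; Each offset lies within plus or minus ShakeDelta, scaled by ShakeAxis, so the shake never drifts and ignores delta time.
; The construction script applies the configurable MaterialInstance to the mesh.
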(event `self.ReceiveBeginPlay`
  (set `self.initialLocation` (`SceneComponent.K2_GetComponentLocation` (`self.StaticMesh`))))

(event `self.ReceiveTick`
  (params (DeltaSeconds :type "Float (single-precision)"))
  (bind _returnvalue (`KismetMathLibrary.Abs` (`self.shakeDelta`)))
  (bind _returnvalue_2 (`KismetMathLibrary.Abs` (`self.shakeDelta`)))
  (bind _returnvalue_3 (`KismetMathLibrary.Abs` (`self.shakeDelta`)))
  (`SceneComponent.K2_SetWorldLocation` (`self.StaticMesh`) (+ (`self.initialLocation`) (`KismetMathLibrary.MakeVector` (* (.x (`self.shakeAxis`)) (`KismetMathLibrary.RandomFloatInRange` (* _returnvalue -1.0) _returnvalue)) (* (.y (`self.shakeAxis`)) (`KismetMathLibrary.RandomFloatInRange` (* _returnvalue_2 -1.0) _returnvalue_2)) (* (.z (`self.shakeAxis`)) (`KismetMathLibrary.RandomFloatInRange` (* _returnvalue_3 -1.0) _returnvalue_3)))) false false))

(fn `UserConstructionScript`
  (`PrimitiveComponent.SetMaterial` (`self.StaticMesh`) 0 (`self.materialInstance`)))